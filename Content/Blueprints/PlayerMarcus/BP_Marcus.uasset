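; BP_Marcus is the player Blueprint for Marcus, and its graph drives a parallax scrolling background.
; On BeginPlay it creates a dynamic material for each Paper2D sprite under StaticBackground and assigns a per-layer multiplier from ParalaxMultiplyers by child index.
; Every Tick it passes the camera's world X to those materials as CameraPosX, so the scrolling is left to the material.
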(event `self.ReceiveBeginPlay`
  ; Paralax Scrolling
  (for (_array_element _array_index) (`SceneComponent.GetChildrenComponents` (`self.Static Background`) false)
    (bind _aspaper_sprite_component (cast `PaperSpriteComponent` _array_element))
    (bind _returnvalue (`PrimitiveComponent.CreateDynamicMaterialInstance` _aspaper_sprite_component 0 null "None"))
    (`KismetArrayLibrary.Array_Add` (`self.DynamicLayers`) _returnvalue)
    (`MaterialInstanceDynamic.SetScalarParameterValue` _returnvalue "Paralax Multiplyer" (`|GetArrayItem` (`self.ParalaxMultiplyers`) _array_index))))

(event `self.ReceiveTick`
  (params (DeltaSeconds :type "Float (single-precision)"))
  (bind _returnvalue_x (`KismetMathLibrary.BreakVector` (`SceneComponent.K2_GetComponentLocation` (`self.Camera`))))
  (for _array_element (`self.DynamicLayers`)
    (`MaterialInstanceDynamic.SetScalarParameterValue` _array_element "CameraPosX" _returnvalue_x)))

(fn `UserConstructionScript`)